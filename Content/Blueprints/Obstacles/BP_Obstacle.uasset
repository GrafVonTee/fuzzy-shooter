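; BP_Obstacle is a cylinder obstacle that supplies a hidden point of interest, apparently a spot shadowed from a given source.
; The Shadowfrom event turns the SpringArm using a look-at rotation between the obstacle and the source's X/Y position.
; It sets the arm length through CalculateNewEllipseRadius from that rotation and the cylinder's world scale, accommodating elliptical footprints.
; GetPointOfInterest returns the HiddenPoint component's world location.
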(event EventBeginPlay)

(event Collision|EventActorBeginOverlap
  (params (OtherActor :type Actor%20Object%20Reference)))

(event EventTick
  (params (DeltaSeconds :type Float%20%28single-precision%29)))

(event EventShadowfrom
  (params (Source :type Vector :default "0, 0, 0"))
  (bind _returnvalue (Transformation|GetActorLocation))
  (bind _springarm (Variables|Default|GetSpringArm))
  (bind _returnvalue_2 (Math|Rotator|FindLookatRotation (Math|Vector|MakeVector (.x _returnvalue) (.y _returnvalue) 0.0) (Math|Vector|MakeVector (.x Source) (.y Source) 0.0)))
  (Transformation|SetWorldRotation _springarm _returnvalue_2 false false)
  (Variables|/Script/Engine.SpringArmComponent|SetTargetArmLength _springarm (Class|Obstacle|CalculateNewEllipseRadius _returnvalue_2 (Transformation|GetWorldScale (Variables|Default|GetCylinder)))))

(fn ConstructionScript)

(fn GetPointOfInterest
  (return (Transformation|GetWorldLocation (Variables|Default|GetHiddenPoint))))