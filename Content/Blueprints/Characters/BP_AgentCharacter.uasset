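; Agent character Blueprint that turns to face targets, shoots at other characters and shows a characteristics widget on screen.
; BeginPlay adds the widget to the viewport, and OnDestroyAction removes it before destroying the actor.
; BeginAttack runs a debug-drawn line trace forward from SpawnPoint, spawning BP_Bullet and spending ammo only when it hits a BaseCharacter.
; Lookat snaps rotation toward a target using X/Y positions, and StopAttack resets the shooting timer.
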(event EventBeginPlay
  (bind _returnvalue (UserInterface|CreateWidget "/Game/Blueprints/HUD/UI_AgentCharacteristics.UI_AgentCharacteristics_C"))
  (bind _output_get (Variables|Default|SetAgentWidget _returnvalue))
  (UserInterface|Viewport|AddtoViewport _output_get 0))

(event Collision|EventActorBeginOverlap
  (params (OtherActor :type Actor%20Object%20Reference)))

(event EventStopAttack
  (Class|AgentCharacter|ResetShootingTimer))

(event EventBeginAttack
  (bind _spawnpoint (Variables|Default|GetSpawnPoint))
  (bind _spawnpoint_2 (Variables|Default|GetSpawnPoint))
  (bind _returnvalue (Transformation|GetWorldLocation _spawnpoint_2))
  (bind _returnvalue_2 (Transformation|GetWorldTransform _spawnpoint))
  (bind _outhit (Collision|LineTraceForObjects _returnvalue (+ (* (Math|Vector|GetForwardVector (Transformation|GetActorRotation)) 1.5e+03) _returnvalue) (Variables|Default|GetObject%20Types) false 0 "ForDuration"))
  (Utilities|Casting|CastToBaseCharacter (.HitActor (Collision|BreakHitResult _outhit)))
  (Game|SpawnActorfromClass "/Game/Blueprints/Characters/BP_Bullet.BP_Bullet_C" (Math|Transform|MakeTransform (.location _returnvalue_2) (.rotation _returnvalue_2) "1,1,1") "AlwaysSpawn" 0 0)
  (Math|Integer|DecrementInt (Variables|Default|GetCurrentAmmo)))

(event EventLookat
  (params (Target :type Vector :default "0, 0, 0"))
  (bind _returnvalue (Transformation|GetActorLocation))
  (Transformation|SetActorRotation (Math|Rotator|FindLookatRotation (Math|Vector|MakeVector (.x _returnvalue) (.y _returnvalue) 0.0) (Math|Vector|MakeVector (.x Target) (.y Target) 0.0))))

(event EventOnDestroyAction
  (Widget|RemovefromParent (Variables|Default|GetAgentWidget))
  (Actor|DestroyActor))

(fn ConstructionScript)