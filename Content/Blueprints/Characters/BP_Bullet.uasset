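; BP_Bullet is a bullet actor that damages characters it hits.
; On BeginPlay it scales its Sphere by SphereSize and destroys itself after a short fixed lifetime.
; A Sphere hit on a BaseCharacter other than CharOwner calls ReceiveDamage with a fixed amount and destroys the bullet.
; Hitting anything that is not a BaseCharacter also destroys it, while hits on CharOwner are ignored.
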(event OnComponentHit(Sphere)
  (params (HitComponent :type Primitive%20Component%20Object%20Reference) (OtherActor :type Actor%20Object%20Reference) (OtherComp :type Primitive%20Component%20Object%20Reference) (NormalImpulse :type Vector :default "0, 0, 0") (Hit :type Hit%20Result%20Structure%20%28by%20ref%29))
  (bind _asbase_character (Utilities|Casting|CastToBaseCharacter OtherActor)
    (:then
      (if (not (== _asbase_character (Variables|Default|GetCharOwner)))
        (Class|BaseCharacter|ReceiveDamage _asbase_character 3)
        (Actor|DestroyActor :!label _label)))
    (:CastFailed
      (goto _label))))

(event EventBeginPlay
  (Transformation|SetRelativeScale3D (Variables|Default|GetSphere) (* "1.000000,1.000000,1.000000" (Variables|Default|GetSphereSize)))
  (Utilities|FlowControl|Delay 3.0)
  (Actor|DestroyActor))

(fn ConstructionScript)