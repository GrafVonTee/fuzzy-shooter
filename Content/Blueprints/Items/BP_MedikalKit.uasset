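; BP_MedikalKit is a consumable medical kit item that heals the character who uses it.
; Its ConsumeItem event adds the item's CurrentValue to the character's CurrentHealth, clamped between zero and MaxHealth.
; BeginPlay and the construction script only call the parent, and the overlap and tick events are disabled.
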(event EventBeginPlay
  (|CallParentFunction))

(event Collision|EventActorBeginOverlap
  (params (OtherActor :type Actor%20Object%20Reference))
  (|CallParentFunction OtherActor) ; This node is disabled and will not be called.\nDrag off pins to build functionality.
)

(event EventTick
  (params (DeltaSeconds :type Float%20%28single-precision%29))
  (|CallParentFunction DeltaSeconds) ; This node is disabled and will not be called.\nDrag off pins to build functionality.
)

(event EventConsumeItem
  (params (Character :type HOTRELOADED%20Base%20Character%201%20Object%20Reference))
  (Variables|/Script/FuzzyShooter.BaseCharacter|SetCurrentHealth Character (Math|Integer|Clamp(Integer) (+ (Variables|/Script/FuzzyShooter.BaseCharacter|GetCurrentHealth Character) (Variables|Default|GetCurrentValue)) 0 (Variables|/Script/FuzzyShooter.BaseCharacter|GetMaxHealth Character))))

(fn ConstructionScript
  (|CallParentFunction))