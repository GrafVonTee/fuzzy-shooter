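; BP_AmmoBox is an item that refills a character's ammo when consumed.
; Its ConsumeItem event adds the item's CurrentValue to the character's CurrentAmmo, clamped between zero and that character's MaxAmmo.
; BeginPlay, overlap and Tick are disabled stubs, and the construction script only calls its parent, so the ammo refill is the only logic defined here.
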(event EventBeginPlay
  (|CallParentFunction) ; This node is disabled and will not be called.\nDrag off pins to build functionality.
)

(event Collision|EventActorBeginOverlap
  (params (OtherActor :type Actor%20Object%20Reference))
  (|CallParentFunction OtherActor) ; This node is disabled and will not be called.\nDrag off pins to build functionality.
)

(event EventTick
  (params (DeltaSeconds :type Float%20%28single-precision%29))
  (|CallParentFunction DeltaSeconds) ; This node is disabled and will not be called.\nDrag off pins to build functionality.
)

(event EventConsumeItem
  (params (Character :type Base%20Character%20Object%20Reference))
  (Variables|/Script/FuzzyShooter.BaseCharacter|SetCurrentAmmo Character (Math|Integer|Clamp(Integer) (+ (Variables|/Script/FuzzyShooter.BaseCharacter|GetCurrentAmmo Character) (Variables|Default|GetCurrentValue)) 0 (Variables|/Script/FuzzyShooter.BaseCharacter|GetMaxAmmo Character))))

(fn ConstructionScript
  (|CallParentFunction))